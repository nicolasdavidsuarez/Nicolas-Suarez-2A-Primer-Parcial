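; Enemy actor that moves continuously and can fire BP_Bala projectiles.
; Tick applies a local offset of normalized velocity times a speed factor, without delta-time scaling or sweep, so speed depends on frame rate.
; Setter functions supply that vector and factor.
; Dispara spawns a bullet at the enemy's transform, multiplying direction, passed speed and a bullet-speed multiplier intended to keep it faster than the enemy.
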(event `self.ReceiveTick`
  (params (DeltaSeconds :type "Float (single-precision)"))
  ;[1 1 1] Movimiento del enemigo
  (`self.K2_AddActorLocalOffset` (* (`self.Velociad Normalizada`) (`self.Factor Velocidad`))))

(fn `Dispara`
  (params (direccion :type "Vector Structure") (velocidad :type "Float (double-precision)"))
  (`|SpawnActorFromClass` "/Game/BP_Bala.BP_Bala_C" (`self.GetTransform`) "Undefined" "MultiplyWithRoot" null (* direccion (* velocidad (`self.Velocidad de bala`))) null))

(fn `set Factor Velocidad`
  (params (factorVelocidad :type "Float (double-precision)"))
  (set `self.Factor Velocidad` factorVelocidad))

(fn `setVectorVelocidad`
  (params (velocidadNormalizada :type "Vector Structure"))
  (set `self.Velociad Normalizada` velocidadNormalizada))

(fn `UserConstructionScript`)