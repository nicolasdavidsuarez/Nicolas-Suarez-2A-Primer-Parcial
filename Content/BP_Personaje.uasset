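; BP_Personaje is a character Blueprint that moves itself every Tick by VelocidadNormalizada times FactorVelocidad, without sweep.
; EsAtacado sets an attacked flag, which Tick checks roughly every two seconds and then resets.
; When flagged, Tick sets a one-second timer for an event that doubles FactorVelocidad but clears it immediately, so that timed speed-up never fires.
; A getter exposes FactorVelocidad.
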(event `self.ReceiveTick`
  (params (DeltaSeconds :type "Float (single-precision)"))
  (set `self.tiempoDeRevision` (+ DeltaSeconds (`self.tiempoDeRevision`)))
  ;[1 1 1] Movimiento del Personaje
  (`self.K2_AddActorLocalOffset` (* (`self.velocidadNormalizada`) (`self.factorVelocidad`)))
  (if (> (`self.tiempoDeRevision`) 2.0)
    (set `self.tiempoDeRevision` 0.0)
    (if (`self.meAtacan`)
      (bind _returnvalue (`KismetSystemLibrary.K2_SetTimerDelegate` (delegate `espera`) 1.0))
      (`KismetSystemLibrary.K2_ClearAndInvalidateTimerHandle` _returnvalue)
      (set `self.meAtacan` false))))

(event `espera`
  (set `self.factorVelocidad` (* (`self.factorVelocidad`) 2.0)))

(fn `esAtacado`
  (set `self.meAtacan` true))

(fn `get FactorVelocidad`
  (returns (factorVelocidad :type "Float (double-precision)"))
  (return (`self.factorVelocidad`)))

(fn `UserConstructionScript`)